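; HUD for an RTS that draws a drag marquee and selects the units inside it.
; Input start either clears an existing selection or, if none exists, begins a marquee at the mouse; hold updates its far corner.
; While drawing, DrawHUD uses GetActorsInSelectionRectangle to accumulate RTS_UnitMaster2 units, marking them selected with decals.
; Input release stops drawing and passes the selected units to RTS_PlayerController_BP.
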(event Custom|DrawMarquee
  (bind _clickedlocation (Variables|MarqueeVariables|GetClickedLocation))
  (bind _holdinglocation (Variables|MarqueeVariables|GetHoldingLocation))
  (bind _clickedlocation_2 (Variables|MarqueeVariables|GetClickedLocation))
  (bind _holdinglocation_2 (Variables|MarqueeVariables|GetHoldingLocation))
  (bind (_x _y) (Math|Vector2D|BreakVector2D _clickedlocation))
  (bind (_x_2 _y_2) (Math|Vector2D|BreakVector2D _holdinglocation))
  (bind (_x_3 _y_3) (Math|Vector2D|BreakVector2D _clickedlocation_2))
  (bind _returnvalue (- _holdinglocation_2 _clickedlocation_2))
  (bind (_x_4 _y_4) (Math|Vector2D|BreakVector2D _returnvalue))
  (HUD|DrawRect "(R=0,G=0,B=0,A=1)" _x _y 0.0 0.0)
  (HUD|DrawRect "(R=0,G=0,B=0,A=1)" _x_2 _y_2 0.0 0.0)
  (HUD|DrawRect "(R=0.091000,G=0.536000,B=0.761000,A=0.600000)" _x_3 _y_3 _x_4 _y_4))

(event EventBeginPlay
  (Variables|References|SetControllerRef (.AsRTS%20Player%20Controller%20BP (Utilities|Casting|CastToRTS_PlayerController_BP (Game|GetPlayerController 0)))))

(event EventDrawHUD
  (params (SizeX :type Integer) (SizeY :type Integer))
  (if (Variables|Bool|GetisDrawing)
    (Utilities|FlowControl|Sequence
      (:then_0
        (CallFunction|DrawMarquee)
        (bind _output_get (Variables|Units|SetUnitsInSelectionArea (Class|HUD|GetActorsinSelectionRectangle "/Game/RTS_Tutorial/Blueprints/Units/RTS_UnitMaster2_Blueprint.RTS_UnitMaster2_Blueprint_C" (Variables|MarqueeVariables|GetClickedLocation) (Variables|MarqueeVariables|GetHoldingLocation) false false)))
        (for _array_element _output_get
          (if (Utilities|ClassIsChildOf (Utilities|GetClass _array_element) "/Game/RTS_Tutorial/Blueprints/Units/RTS_UnitMaster2_Blueprint.RTS_UnitMaster2_Blueprint_C")
            (bind _asrts_unit_master_2_blueprint (Utilities|Casting|CastToRTS_UnitMaster2_Blueprint _array_element))
            (Variables|Units|SetSelectedUnit _asrts_unit_master_2_blueprint)
            (Utilities|FlowControl|Sequence
              (:then_0
                (Utilities|Array|AddUnique (Variables|Units|GetSelectedUnits) (Variables|Units|GetSelectedUnit)))
              (:then_1
                (for _array_element_2 (Variables|Units|GetSelectedUnits)
                  (Default|SetSelectedDecal _array_element_2)
                  (Variables|/Game/RTS_Tutorial/Blueprints/Units/RTS_UnitMaster2_Blueprint.RTS_UnitMaster2_Blueprint_C|SetisSelected _array_element_2 true))))))))))

(event EventOnInputHold
  (bind _controllerref (Variables|References|GetControllerRef))
  (bind (_locationx _locationy) (Game|Player|GetMousePosition _controllerref))
  (Variables|MarqueeVariables|SetHoldingLocation (Math|Vector2D|MakeVector2D _locationx _locationy)))

(event EventOnInputStart
  (bind _controllerref (Variables|References|GetControllerRef))
  (bind (_locationx _locationy) (Game|Player|GetMousePosition _controllerref))
  (if (>= (Utilities|Array|LastIndex (Variables|Units|GetSelectedUnits)) 0)
    (for _array_element (Variables|Units|GetSelectedUnits)
      (Default|SetDeselectedDecal _array_element)
      (Variables|/Game/RTS_Tutorial/Blueprints/Units/RTS_UnitMaster2_Blueprint.RTS_UnitMaster2_Blueprint_C|SetisSelected _array_element false)
      (Variables|/Game/RTS_Tutorial/Blueprints/Player/RTS_PlayerController_BP.RTS_PlayerController_BP_C|SetisUnitSelected (Variables|References|GetControllerRef) false))
    (Utilities|Array|Clear (Variables|Units|GetSelectedUnits))
    (else
      (bind _output_get (Variables|MarqueeVariables|SetClickedLocation (Math|Vector2D|MakeVector2D _locationx _locationy)))
      (Variables|MarqueeVariables|SetHoldingLocation _output_get)
      (Variables|Bool|SetisDrawing true))))

(event EventOnInputRelease
  (params (HoldTime :type Float%20%28single-precision%29))
  (Variables|Bool|SetisDrawing false)
  (Default|SetSelectedUnits (Variables|References|GetControllerRef) (Variables|Units|GetSelectedUnits)))

(fn ConstructionScript)