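; RTS player controller that drives the camera pawn's movement, zoom and rotation and shows the mouse cursor.
; On BeginPlay it caches the RTS_CameraPawn_BP reference, then feeds movement axes to its FloatingPawnMovement along world X/Y.
; Zoom inputs adjust spring arm length within limits or reset it.
; Holding Pan blocks movement while mouse input rotates yaw through a gate and clamped pitch through a flag; PanReset zeroes only pitch.
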(event EventBeginPlay
  (Utilities|FlowControl|Sequence
    (:then_0
      (Utilities|ReferenceCast))
    (:then_1
      (Variables|Default|SetbShowMouseCursor true))))

(event Input|ActionEvents|InputActionZoomReset
  (params (Key :type Key%20Structure))
  ;[1 1 1] Zoom Controls
  ;;[1 1 1] Reset Zoom
  (:Pressed
    (Variables|/Script/Engine.SpringArmComponent|SetTargetArmLength (Variables|/Game/RTS_Tutorial/Blueprints/RTS_CameraPawn_BP.RTS_CameraPawn_BP_C|GetSpringArm (Variables|References|GetCameraPawnRef)) 1.5e+03)))

(event Input|ActionEvents|InputActionZoomIn
  (params (Key :type Key%20Structure))
  (bind _camerapawnref (Variables|References|GetCameraPawnRef))
  (bind _springarm (Variables|/Game/RTS_Tutorial/Blueprints/RTS_CameraPawn_BP.RTS_CameraPawn_BP_C|GetSpringArm _camerapawnref))
  ;[1 1 1] Zoom Controls
  ;;[1 1 1] Zoom In
  (:Pressed
    (Variables|/Script/Engine.SpringArmComponent|SetTargetArmLength _springarm (Math|Float|Clamp(Float) (- (Variables|/Script/Engine.SpringArmComponent|GetTargetArmLength _springarm) (Variables|MovementVariables|GetZoomSpeed)) (Variables|MovementVariables|GetMinZoomLimit) (Variables|MovementVariables|GetMaxZoomLimit)))))

(event Input|ActionEvents|InputActionPan
  (params (Key :type Key%20Structure))
  (:Pressed
    (Variables|Bool|SetisPressed true)
    (Variables|Bool|SetDisableCamMovement true))
  (:Released
    (Variables|Bool|SetisPressed false)
    (Variables|Bool|SetDisableCamMovement false)))

(event Input|ActionEvents|InputActionZoomOut
  (params (Key :type Key%20Structure))
  (bind _camerapawnref (Variables|References|GetCameraPawnRef))
  (bind _springarm (Variables|/Game/RTS_Tutorial/Blueprints/RTS_CameraPawn_BP.RTS_CameraPawn_BP_C|GetSpringArm _camerapawnref))
  ;[1 1 1] Zoom Controls
  ;;[1 1 1] Zoom Out
  (:Pressed
    (Variables|/Script/Engine.SpringArmComponent|SetTargetArmLength _springarm (Math|Float|Clamp(Float) (+ (Variables|MovementVariables|GetZoomSpeed) (Variables|/Script/Engine.SpringArmComponent|GetTargetArmLength _springarm)) (Variables|MovementVariables|GetMinZoomLimit) (Variables|MovementVariables|GetMaxZoomLimit)))))

(event Input|ActionEvents|InputActionPan
  (params (Key :type Key%20Structure))
  (bind _camerapawnref (Variables|References|GetCameraPawnRef))
  (bind _returnvalue (Transformation|GetActorRotation _camerapawnref))
  (bind (_roll _pitch _yaw) (Math|Rotator|BreakRotator _returnvalue))
  (:Pressed
    (Variables|Bool|SetDisableCamMovement true)
    (Utilities|FlowControl|Gate true) ; enters at Open
  )
  (:Released
    (Variables|Bool|SetDisableCamMovement false)
    (Utilities|FlowControl|Gate true) ; enters at Close
  ))

(event Input|ActionEvents|InputActionPanReset
  (params (Key :type Key%20Structure))
  (bind _camerapawnref (Variables|References|GetCameraPawnRef))
  (bind _returnvalue (Transformation|GetActorRotation _camerapawnref))
  (bind (_roll _pitch _yaw) (Math|Rotator|BreakRotator _returnvalue))
  ;[1 1 1] Reset Pan
  (:Pressed
    (Transformation|SetActorRotation _camerapawnref (Math|Rotator|MakeRotator _roll 0.0 _yaw))))

(event Input|AxisEvents|InputAxisMoveForward
  (params (AxisValue :type Float%20%28single-precision%29))
  (if (not (Variables|Bool|GetDisableCamMovement))
    (Class|PawnMovementComponent|AddInputVector (Variables|/Game/RTS_Tutorial/Blueprints/RTS_CameraPawn_BP.RTS_CameraPawn_BP_C|GetFloatingPawnMovement (Variables|References|GetCameraPawnRef)) (Math|Vector|MakeVector AxisValue 0.0 0.0) false)))

(event Input|AxisEvents|InputAxisMoveRight
  (params (AxisValue :type Float%20%28single-precision%29))
  (if (not (Variables|Bool|GetDisableCamMovement))
    (Class|PawnMovementComponent|AddInputVector (Variables|/Game/RTS_Tutorial/Blueprints/RTS_CameraPawn_BP.RTS_CameraPawn_BP_C|GetFloatingPawnMovement (Variables|References|GetCameraPawnRef)) (Math|Vector|MakeVector 0.0 AxisValue 0.0) false)))

(event Input|MouseEvents|MouseX
  (params (AxisValue :type Float%20%28single-precision%29))
  (bind _camerapawnref (Variables|References|GetCameraPawnRef))
  (bind _returnvalue (Transformation|GetActorRotation _camerapawnref))
  (bind (_roll _pitch _yaw) (Math|Rotator|BreakRotator _returnvalue))
  (Utilities|FlowControl|Gate true
    (:Exit
      (Transformation|SetActorRotation _camerapawnref (Math|Rotator|MakeRotator _roll _pitch (+ _yaw (* AxisValue (Variables|MovementVariables|GetPanSpeed))))))))

(event Input|MouseEvents|MouseY
  (params (AxisValue :type Float%20%28single-precision%29))
  (bind _camerapawnref (Variables|References|GetCameraPawnRef))
  (bind _returnvalue (Transformation|GetActorRotation _camerapawnref))
  (bind (_roll _pitch _yaw) (Math|Rotator|BreakRotator _returnvalue))
  (if (Variables|Bool|GetisPressed)
    (Transformation|SetActorRotation _camerapawnref (Math|Rotator|MakeRotator _roll (Math|Float|Clamp(Float) (+ _pitch (* AxisValue (Variables|MovementVariables|GetPanSpeed))) 0.0 45.0) _yaw))))

(fn ConstructionScript)